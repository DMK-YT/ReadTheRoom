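; Note actor that shows on-screen widgets while the player character is inside its Box trigger.
; BeginPlay creates the BP_E interact prompt, which the overlap events add and remove.
; Entering also creates and shows a BP_Text note widget, removed on exit, but both steps require BPTextWidgetRef, never assigned here, to cast to Character.
; OnInteract is empty, so the note display is driven by overlap alone.
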(event OnComponentBeginOverlap(Box)
  (params (OverlappedComponent :type Primitive%20Component%20Object%20Reference) (OtherActor :type Actor%20Object%20Reference) (OtherComp :type Primitive%20Component%20Object%20Reference) (OtherBodyIndex :type Integer) (bFromSweep :type Boolean) (SweepResult :type Hit%20Result%20Structure%20%28by%20ref%29))
  (if (== OtherActor (Game|GetPlayerCharacter 0))
    (UserInterface|Viewport|AddtoViewport (Variables|Default|GetInteractwithE) 0)
    (bind _ascharacter (Utilities|Casting|CastToCharacter (Variables|Default|GetBP_TextWidgetRef)))
    (Utilities|IsValid _ascharacter
      (:Is%20Valid
        (bind _returnvalue (UserInterface|CreateWidget "/Game/Blueprints/BP_Text.BP_Text_C"))
        (bind _output_get (Variables|Default|SetNoteWidgetRef _returnvalue))
        (UserInterface|Viewport|AddtoViewport _output_get 0)))))

(event OnComponentEndOverlap(Box)
  (params (OverlappedComponent :type Primitive%20Component%20Object%20Reference) (OtherActor :type Actor%20Object%20Reference) (OtherComp :type Primitive%20Component%20Object%20Reference) (OtherBodyIndex :type Integer))
  (if (== (Game|GetPlayerCharacter 0) OtherActor)
    (Widget|RemovefromParent (Variables|Default|GetInteractwithE))
    (Utilities|Casting|CastToCharacter (Variables|Default|GetBP_TextWidgetRef))
    (Utilities|IsValid (Variables|Default|GetNoteWidgetRef)
      (:Is%20Valid
        (Widget|RemovefromParent (Variables|Default|GetNoteWidgetRef))
        (Variables|Default|SetNoteWidgetRef 0)))))

(event Collision|EventActorBeginOverlap
  (params (OtherActor :type Actor%20Object%20Reference)))

(event EventTick
  (params (DeltaSeconds :type Float%20%28single-precision%29)))

(event EventOnInteract)

(event EventBeginPlay
  (bind _returnvalue (UserInterface|CreateWidget "/Game/Blueprints/BP_E.BP_E_C"))
  (Variables|Default|SetInteractwithE _returnvalue))

(fn ConstructionScript)