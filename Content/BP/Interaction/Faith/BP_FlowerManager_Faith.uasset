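; Flower-collection manager for a bouquet puzzle that shows the remaining flower count on a text display.
; CountFlower tallies flowers as they are picked up, and OnInteract subtracts that tally from the total and resets it.
; When none remain, it moves PaolaKey to a stored position, shows "Bouquet Made" and disables its box collision.
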(event Custom|CountFlower
  (Variables|Default|SetflowerCount (+ (Variables|Default|GetflowerCount) 1)))

(event EventOnInteract
  (Variables|Default|SettotalFlowerCount (- (Variables|Default|GettotalFlowerCount) (Variables|Default|GetflowerCount)))
  (Variables|Default|SetflowerCount 0)
  (if (<= (Variables|Default|GettotalFlowerCount) 0)
    (Transformation|SetActorTransform (Variables|Default|GetpaolaKey) (Math|Transform|MakeTransform (Math|Vector|MakeVector (Variables|Default|GetxPos) (Variables|Default|GetyPos) (Variables|Default|GetzPos)) "0, 0, 0" "1.000000,1.000000,1.000000"))
    (Rendering|Components|TextRender|SetText (Variables|Default|GetTextRender) (Utilities|Text|ToText(String) (Utilities|String|MakeLiteralString "Bouquet Made ")))
    (Collision|SetCollisionEnabled (Variables|Default|GetBox) "NoCollision")
    (else
      (Rendering|Components|TextRender|SetText (Variables|Default|GetTextRender) (Utilities|Text|ToText(String) (Utilities|String|Append (Utilities|String|MakeLiteralString "Flowers Remaining:  ") (Utilities|String|ToString(Integer) (Variables|Default|GettotalFlowerCount))))))))

(event EventBeginPlay
  (Rendering|Components|TextRender|SetText (Variables|Default|GetTextRender) (Utilities|Text|ToText(String) (Utilities|String|Append (Utilities|String|MakeLiteralString "Flowers Remaining:  ") (Utilities|String|ToString(Integer) (Variables|Default|GettotalFlowerCount))))))

(fn ConstructionScript)