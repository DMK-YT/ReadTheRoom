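; BP_Door_Dirk is an interactable door that stays shut while locked, then swings open once and falls over.
; OnKeyCollect clears the lock, and the first unlocked OnInteract disables the box collision and starts the opening timeline.
; That timeline yaws the DoorHinge to DoorOpenVal, then chains into a second timeline that lerps the hinge's rotation and location to fake the fall without physics.
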(event Custom|OnKeyCollect
  (Variables|Default|SetisLocked false))

(event EventOnInteract
  (bind _doorhinge (Variables|Default|GetDoorHinge))
  (if (not (Variables|Default|GetisLocked))
    (if (not (Variables|Default|GetisOpened))
      (Variables|Default|SetisOpened true)
      (Collision|SetCollisionEnabled (Variables|Default|GetBox) "NoCollision")
      (bind _dooropening (Timeline|DoorOpen%20Timeline PlayFromStart)
        (:Update
          (Transformation|SetRelativeRotation (Variables|Default|GetDoorHinge) (Math|Rotator|MakeRotator 0.0 0.0 (Math|Float|Lerp 0.0 (Variables|Default|GetDoorOpenVal) _dooropening)) false false))
        (:Finished
          (bind _doorfalling (Timeline|Timeline PlayFromStart)
            (:Update
              (Transformation|SetRelativeRotation _doorhinge (Math|Rotator|MakeRotator (Math|Float|Lerp 0.0 -9e+01 _doorfalling) 0.0 (Math|Float|Lerp (Variables|Default|GetDoorOpenVal) (- (Variables|Default|GetDoorOpenVal) 4.0) _doorfalling)) false false)
              (Transformation|SetRelativeLocation _doorhinge (Math|Vector|MakeVector -1e+02 (Math|Float|Lerp 0.0 -1.3e+02 _doorfalling) (Math|Float|Lerp 0.0 -145.0 _doorfalling)) false false))))))))

(fn ConstructionScript)