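; BP_Door2 is an interactable keypad door that slides vertically once the Correct flag is set.
; Interacting opens the keypad through BP_Character, showing the cursor and switching to UI-only input, unless it is already open or solved.
; OnDoorCheck closes the keypad, restores game input and disables Box collision regardless of result.
; If Correct, it then plays a timeline driving the door's relative Z.
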(event Custom|OnDoorCheck
  (CallFunction|CloseKeypad)
  (Collision|SetCollisionEnabled (Variables|Default|GetBox) "NoCollision")
  (if (Variables|Default|GetCorrect?)
    (bind _doormovement (Timeline|Timeline_0 PlayFromStart)
      (:Update
        (Transformation|SetRelativeLocation (Variables|Default|GetDoor) (Math|Vector|MakeVector 0.0 0.0 _doormovement) false false)))))

(event Custom|CloseKeypad
  (bind _returnvalue (Game|GetPlayerController 0))
  (Variables|Default|SetisKeypadOpen false)
  (bind _asbp_character (Utilities|Casting|CastToBP_Character (Game|GetPlayerCharacter 0)))
  (Default|EnableKeypad _asbp_character false)
  (Variables|/Script/Engine.PlayerController|SetbShowMouseCursor _returnvalue false)
  (Input|SetInputModeGameOnly _returnvalue true))

(event Custom|OpenKeypad
  (bind _returnvalue (Game|GetPlayerController 0))
  (if (not (Variables|Default|GetCorrect?))
    (Variables|Default|SetisKeypadOpen true)
    (bind _asbp_character (Utilities|Casting|CastToBP_Character (Game|GetPlayerCharacter 0)))
    (Default|EnableKeypad _asbp_character true)
    (Variables|/Script/Engine.PlayerController|SetbShowMouseCursor _returnvalue true)
    (Input|SetInputModeUIOnly _returnvalue 0 "DoNotLock" true)))

(event EventOnInteract
  (if (not (Variables|Default|GetisKeypadOpen))
    (CallFunction|OpenKeypad)))

(fn ConstructionScript)