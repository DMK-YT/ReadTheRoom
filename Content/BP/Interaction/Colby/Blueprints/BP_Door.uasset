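; BP_Door is a key card door that slides along Z when a BP_Character holding the key enters its trigger box.
; Begin overlap checks HasKey, then plays the DoorMovement timeline to drive the door's relative Z, or prints a locked message.
; End overlap repeats the key check and reverses a second, separate timeline from its end, so an interrupted movement does not resume from its current position.
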(event OnComponentBeginOverlap(Box)
  (params (OverlappedComponent :type Primitive%20Component%20Object%20Reference) (OtherActor :type Actor%20Object%20Reference) (OtherComp :type Primitive%20Component%20Object%20Reference) (OtherBodyIndex :type Integer) (bFromSweep :type Boolean) (SweepResult :type Hit%20Result%20Structure%20%28by%20ref%29))
  (bind _asbp_character (Utilities|Casting|CastToBP_Character OtherActor))
  (if (Variables|/Game/BP/BP_Character.BP_Character_C|GetHasKey? _asbp_character)
    (bind _doormovement (Timeline|DoorMovement PlayFromStart)
      (:Update
        (Transformation|SetRelativeLocation (Variables|Default|GetDoor) (Math|Vector|MakeVector 0.0 0.0 _doormovement) false false)))
    (else
      (Development|PrintString "Door Locked! Key card required!"))))

(event OnComponentEndOverlap(Box)
  (params (OverlappedComponent :type Primitive%20Component%20Object%20Reference) (OtherActor :type Actor%20Object%20Reference) (OtherComp :type Primitive%20Component%20Object%20Reference) (OtherBodyIndex :type Integer))
  (bind _asbp_character (Utilities|Casting|CastToBP_Character OtherActor))
  (if (Variables|/Game/BP/BP_Character.BP_Character_C|GetHasKey? _asbp_character)
    (bind _doormovement (Timeline|Timeline ReverseFromEnd)
      (:Update
        (Transformation|SetRelativeLocation (Variables|Default|GetDoor) (Math|Vector|MakeVector 0.0 0.0 _doormovement) false false)))))

(fn ConstructionScript)