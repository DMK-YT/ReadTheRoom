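; BP_Note is an interactable note that shows a text widget on screen.
; OnInteract creates the widget, adds it to the viewport and sets IsOpen to block duplicates.
; When a BP_Character leaves the Box collision, it removes the valid widget, clears the reference and resets IsOpen so the note can open again.
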(event OnComponentEndOverlap(Box)
  (params (OverlappedComponent :type Primitive%20Component%20Object%20Reference) (OtherActor :type Actor%20Object%20Reference) (OtherComp :type Primitive%20Component%20Object%20Reference) (OtherBodyIndex :type Integer))
  (Utilities|Casting|CastToBP_Character OtherActor)
  (Utilities|IsValid (Variables|Default|GetNoteWidgetRef)
    (:Is%20Valid
      (Widget|RemovefromParent (Variables|Default|GetNoteWidgetRef))
      (Variables|Default|SetNoteWidgetRef 0)
      (Variables|Default|SetisOpen false))))

(event Collision|EventActorBeginOverlap
  (params (OtherActor :type Actor%20Object%20Reference)))

(event EventTick
  (params (DeltaSeconds :type Float%20%28single-precision%29)))

(event EventOnInteract
  (if (not (Variables|Default|GetisOpen))
    (bind _returnvalue (UserInterface|CreateWidget "/Game/BP/Interaction/Paola/BP_Text.BP_Text_C"))
    (bind _output_get (Variables|Default|SetNoteWidgetRef _returnvalue))
    (UserInterface|Viewport|AddtoViewport _output_get 0)
    (Variables|Default|SetisOpen true)))

(fn ConstructionScript)