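; BP_default is an interactable object that is destroyed on use and can drop a key to another room.
; On interact, it increments the Objectsdestroy counter on the player's BP_Character, so progress is shared through the character.
; Once that count is at least seven, it spawns BP_key_to_other_room at its own location before destroying itself.
; The threshold is not an exact match, so any further interactions past it also spawn keys.
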(event EventOnInteract
  (bind _asbp_character (Utilities|Casting|CastToBP_Character (Game|GetPlayerCharacter 0)))
  (Math|Integer|IncrementInt (Variables|/Game/BP/BP_Character.BP_Character_C|GetObjectsdestroy _asbp_character)
    (:%20%20
      (if (>= (Variables|/Game/BP/BP_Character.BP_Character_C|GetObjectsdestroy _asbp_character) 7)
        (Game|SpawnActorfromClass "/Game/BP/Interaction/Dylan/BP_key_to_other_room.BP_key_to_other_room_C" (Math|Transform|MakeTransform (Transformation|GetActorLocation)) "Undefined" "MultiplyWithRoot" 0 0)
        (Actor|DestroyActor)
        (else
          (Actor|DestroyActor))))))

(fn ConstructionScript)