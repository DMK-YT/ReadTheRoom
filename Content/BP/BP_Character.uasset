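; Player character with Enhanced Input walking, looking and sprinting, plus overlap-based interaction.
; Counts overlapping BPI_Interaction actors to toggle the UI interact alert, and the interact key messages all of them.
; Creates the HUD, note and keypad widgets at BeginPlay, exposing events to set and show notes or toggle keypad opacity; Escape closes notes.
; Destruction calls OpenLevel with the level name "None".
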(event Custom|EnableKeypad
  (params (bool :type Boolean))
  (bind _keypin (Variables|Default|GetKeypin))
  (if bool
    (Widget|SetRenderOpacity _keypin 1.0)
    (else
      (Widget|SetRenderOpacity _keypin 0.0))))

(event Custom|DisplayNote
  ;[0.15 0.15 0.15 0.5] Notes Display
  (if (not (Variables|Default|GetIsDisplayingNote))
    (Default|DisplayWidget (Variables|Default|GetWI_Note) true)
    (Variables|Default|SetIsDisplayingNote true)))

(event Custom|TextToWidget
  (params (NewParam :type String))
  ;[0.15 0.15 0.15 0.5] Notes Display
  (Default|SetDisplayText (Variables|Default|GetWI_Note) NewParam))

(event Input|EnhancedActionEvents|EnhancedInputActionIA_Locomotion
  (params (ActionValue :type Float%20%28double-precision%29) (ElapsedSeconds :type Float%20%28double-precision%29) (TriggeredSeconds :type Float%20%28double-precision%29) (InputAction :type Input%20Action%20Object%20Reference :default "/Game/BP/UserInput/IO/IA_Locomotion.IA_Locomotion"))
  (Pawn|Input|AddMovementInput (Transformation|GetActorForwardVector) ActionValue false))

(event Input|EnhancedActionEvents|EnhancedInputActionIA_LookH
  (params (ActionValue :type Float%20%28double-precision%29) (ElapsedSeconds :type Float%20%28double-precision%29) (TriggeredSeconds :type Float%20%28double-precision%29) (InputAction :type Input%20Action%20Object%20Reference :default "/Game/BP/UserInput/IO/IA_LookH.IA_LookH"))
  (Pawn|Input|AddControllerYawInput ActionValue))

(event Input|EnhancedActionEvents|EnhancedInputActionIA_LookV
  (params (ActionValue :type Float%20%28double-precision%29) (ElapsedSeconds :type Float%20%28double-precision%29) (TriggeredSeconds :type Float%20%28double-precision%29) (InputAction :type Input%20Action%20Object%20Reference :default "/Game/BP/UserInput/IO/IA_LookV.IA_LookV"))
  (Pawn|Input|AddControllerPitchInput ActionValue))

(event Input|EnhancedActionEvents|EnhancedInputActionIA_Strafe
  (params (ActionValue :type Float%20%28double-precision%29) (ElapsedSeconds :type Float%20%28double-precision%29) (TriggeredSeconds :type Float%20%28double-precision%29) (InputAction :type Input%20Action%20Object%20Reference :default "/Game/BP/UserInput/IO/IA_Strafe.IA_Strafe"))
  (Pawn|Input|AddMovementInput (Transformation|GetActorRightVector) ActionValue false))

(event Input|EnhancedActionEvents|EnhancedInputActionIA_Sprint
  (params (ActionValue :type Boolean) (ElapsedSeconds :type Float%20%28double-precision%29) (TriggeredSeconds :type Float%20%28double-precision%29) (InputAction :type Input%20Action%20Object%20Reference :default "/Game/BP/UserInput/IO/IA_Sprint.IA_Sprint"))
  (bind _charactermovement (Variables|Character|GetCharacterMovement))
  (bind _defaultmovespeed (Variables|Default|GetdefaultMoveSpeed))
  (:Started
    (Variables|/Script/Engine.CharacterMovementComponent|SetMaxWalkSpeed _charactermovement (* (Variables|Default|GetsprintSpeedMultiplier) _defaultmovespeed)))
  (:Completed
    (Variables|/Script/Engine.CharacterMovementComponent|SetMaxWalkSpeed _charactermovement _defaultmovespeed)))

(event Input|EnhancedActionEvents|EnhancedInputActionIA_Interact
  (params (ActionValue :type Boolean) (ElapsedSeconds :type Float%20%28double-precision%29) (TriggeredSeconds :type Float%20%28double-precision%29) (InputAction :type Input%20Action%20Object%20Reference :default "/Game/BP/UserInput/IO/IA_Interact.IA_Interact"))
  ;[0.15 0.15 0.15 0.5] Player Interaction
  (:Started
    (for _array_element (Collision|GetOverlappingActors 0 :!class /Script/Engine.Actor)
      (if (Utilities|DoesObjectImplementInterface _array_element "/Game/BP/Interaction/BPI_Interaction.BPI_Interaction_C")
        (Class|BPIInteraction|OnInteract(Message) _array_element)))))

(event Input|EnhancedActionEvents|EnhancedInputActionIA_Escape
  (params (ActionValue :type Boolean) (ElapsedSeconds :type Float%20%28double-precision%29) (TriggeredSeconds :type Float%20%28double-precision%29) (InputAction :type Input%20Action%20Object%20Reference :default "/Game/BP/UserInput/IO/IA_Escape.IA_Escape"))
  (:Started
    (if (Variables|Default|GetIsDisplayingNote)
      (Default|DisplayWidget (Variables|Default|GetWI_Note) false)
      (Variables|Default|SetIsDisplayingNote false))))

(event EventBeginPlay
  (Input|AddMappingContext (PlayerController|LocalPlayerSubsystems|GetEnhancedInputLocalPlayerSubsystem (Game|GetPlayerController 0)) "/Game/BP/UserInput/IO/IMC_BaseCharacter.IMC_BaseCharacter" 0 "(bIgnoreAllPressedKeysUntilRelease=True,bForceImmediately=False,bNotifyUserSettings=False)")
  (Variables|Default|SetdefaultMoveSpeed (Variables|/Script/Engine.CharacterMovementComponent|GetMaxWalkSpeed (Variables|Character|GetCharacterMovement)))
  (bind _returnvalue (UserInterface|CreateWidget "/Game/UI/WB_UI.WB_UI_C"))
  (bind _output_get (Variables|Default|SetUI _returnvalue))
  (UserInterface|Viewport|AddtoViewport _output_get 0)
  (bind _returnvalue_2 (UserInterface|CreateWidget "/Game/BP/Interaction/Colby/Blueprints/WI_Note.WI_Note_C"))
  (bind _output_get_2 (Variables|Default|SetWI_Note _returnvalue_2))
  (UserInterface|Viewport|AddtoViewport _output_get_2 0)
  (bind _aswi_note (Utilities|Casting|CastToWI_Note _returnvalue_2))
  (Default|DisplayWidget _aswi_note false)
  (bind _returnvalue_3 (UserInterface|CreateWidget "/Game/BP/Interaction/Colby/Blueprints/Keypad_WB.Keypad_WB_C"))
  (bind _output_get_3 (Variables|Default|SetKeypin _returnvalue_3))
  (UserInterface|Viewport|AddtoViewport _output_get_3 0)
  (bind _askeypad_wb (Utilities|Casting|CastToKeypad_WB _returnvalue_3))
  (Widget|SetRenderOpacity _askeypad_wb 0.0))

(event Collision|EventActorBeginOverlap
  (params (OtherActor :type Actor%20Object%20Reference))
  ;[0.15 0.15 0.15 0.5] Player Interaction
  (if (Utilities|DoesObjectImplementInterface OtherActor "/Game/BP/Interaction/BPI_Interaction.BPI_Interaction_C")
    (Default|TriggerInteractAlert (Variables|Default|GetUI) true)
    (Variables|Default|SetcurrentInteractiblesCount (Math|Integer|Clamp(Integer) (+ (Variables|Default|GetcurrentInteractiblesCount) 1) 0 99999))))

(event Collision|EventActorEndOverlap
  (params (OtherActor :type Actor%20Object%20Reference))
  ;[0.15 0.15 0.15 0.5] Player Interaction
  (if (Utilities|DoesObjectImplementInterface OtherActor "/Game/BP/Interaction/BPI_Interaction.BPI_Interaction_C")
    (bind _output_get (Variables|Default|SetcurrentInteractiblesCount (Math|Integer|Clamp(Integer) (+ (Variables|Default|GetcurrentInteractiblesCount) -1) 0 99999)))
    (if (not (> _output_get 0))
      (Default|TriggerInteractAlert (Variables|Default|GetUI) false))))

(event EventDestroyed
  (Game|OpenLevel(byName) "None"))

(fn ConstructionScript)